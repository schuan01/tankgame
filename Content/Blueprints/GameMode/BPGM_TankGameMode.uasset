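; Game mode for a tank game that spawns the enemies and counts how many are destroyed.
; On BeginPlay it spawns a BP_Enemy at the transform of every BP_EnemySpawnLocation actor and binds to each one's OnEnemyDestroyed event.
; Each destruction increments EnemyCount, which acts as a kill tally rather than a remaining count, and prints it for debugging.
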(event Custom|UpdateEnemyCount
  (Math|Integer|IncrementInt (Variables|Default|GetenemyCount)))

(event Custom|EnemyDestroyed
  (CallFunction|UpdateEnemyCount)
  (Development|PrintString (Utilities|String|ToString(Integer) (Variables|Default|GetenemyCount))))

(event EventBeginPlay
  (bind _outactors (Actor|GetAllActorsOfClass "/Game/Blueprints/Enemy/BP_EnemySpawnLocation.BP_EnemySpawnLocation_C"))
  (for _array_element _outactors
    (bind _returnvalue (Game|SpawnActorfromClass "/Game/Blueprints/Enemy/BP_Enemy.BP_Enemy_C" (Transformation|GetActorTransform _array_element) "Undefined" 0 0))
    (EventDispatchers|BindEventtoOnEnemyDestroyed _returnvalue (delegate Custom|EnemyDestroyed))))

(event EventTick
  (params (DeltaSeconds :type Float%20%28single-precision%29)))

(fn ConstructionScript)