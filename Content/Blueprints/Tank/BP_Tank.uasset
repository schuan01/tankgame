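; BP_Tank is a tank actor whose gun aims at the mouse cursor and fires projectiles on left click.
; BeginPlay shows the mouse cursor, and each Tick yaws GunCenter toward the visibility trace hit under it, keeping pitch and roll.
; Left mouse press calls ShootProjectile, which spawns a scaled-down BP_TankProjectile at the SpawnLocation component's position and rotation.
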(event Custom|ShootProjectile
  (bind _spawnlocation (Variables|Default|GetSpawnLocation))
  (Game|SpawnActorfromClass "/Game/Blueprints/Projectile/BP_TankProjectile.BP_TankProjectile_C" (Math|Transform|MakeTransform (Transformation|GetWorldLocation _spawnlocation) (Transformation|GetWorldRotation _spawnlocation) "0.200000,0.200000,0.200000") "Undefined" 0 0))

(event EventBeginPlay
  (Variables|/Script/Engine.PlayerController|SetbShowMouseCursor (Game|GetPlayerController 0) true))

(event Collision|EventActorBeginOverlap
  (params (OtherActor :type Actor%20Object%20Reference)))

(event EventTick
  (params (DeltaSeconds :type Float%20%28single-precision%29))
  (bind _guncenter (Variables|Default|GetGunCenter))
  (bind _returnvalue (Transformation|GetWorldRotation _guncenter))
  (Transformation|SetWorldRotation _guncenter (Math|Rotator|MakeRotator (.roll _returnvalue) (.pitch _returnvalue) (.yaw (Math|Rotator|FindLookatRotation (Transformation|GetWorldLocation (Variables|Default|GetGunCenter)) (.Location (Collision|BreakHitResult (.HitResult (Game|Player|GetHitResultUnderCursorbyChannel (Game|GetPlayerController 0) "TraceTypeQuery1" true))))))) false false))

(event Input|MouseEvents|LeftMouseButton
  (params (Key :type Key%20Structure :default "None"))
  (:Pressed
    (CallFunction|ShootProjectile)))

(fn ConstructionScript)